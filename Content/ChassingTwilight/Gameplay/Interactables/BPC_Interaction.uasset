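; Interaction component that lets its owner use objects implementing BPI_Interaction that the player looks at.
; Each tick it line-traces a short distance from the player camera, caches the hit interactable and shows or hides its prompt in WB_Interaction, found on BeginPlay.
; Interact messages that actor locally, then repeats the message through SRInteract with the ServerInteract flag set, separating local and server responses.
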(event Custom|Interact
  (Variables|Default|GetIntereact%20Actor
    (:then
      (Class|BPIInteraction|Interact(Message) (Variables|Default|GetIntereact%20Actor) (Components|GetOwner) false)
      (CallFunction|SRInteract (Variables|Default|GetIntereact%20Actor) (Components|GetOwner)))
    (:else)))

(event Custom|SR%20Interact
  (params (Target :type Actor%20Object%20Reference) (Player%20That%20Interracts :type Actor%20Object%20Reference))
  (Class|BPIInteraction|Interact(Message) Target Player%20That%20Interracts true))

(event EventBeginPlay
  (bind _widgetref (Utilities|GetWidgetReference "/Game/ChassingTwilight/Gameplay/Interactables/WB_Interaction.WB_Interaction_C" 10)
    (:true
      (bind _aswb_interaction (Utilities|Casting|CastToWB_Interaction _widgetref))
      (Variables|Default|SetAs%20WB%20Interaction _aswb_interaction))))

(event EventTick
  (params (DeltaSeconds :type Float%20%28single-precision%29))
  (CallFunction|InteractionTrace))

(fn InteractionTrace
  (bind _returnvalue (Game|GetPlayerCameraManager 0))
  (bind _returnvalue_2 (Transformation|GetActorLocation _returnvalue))
  (bind (_outhit _returnvalue_3) (Collision|LineTraceByChannel _returnvalue_2 (+ _returnvalue_2 (* (Transformation|GetActorForwardVector _returnvalue) 2.5e+02)) "TraceTypeQuery1" false 0 "None"))
  (if _returnvalue_3
    (if (Utilities|DoesObjectImplementInterface (.HitActor (Collision|BreakHitResult _outhit)) "/Game/ChassingTwilight/Gameplay/Interactables/BPI_Interaction.BPI_Interaction_C")
      (bind _output_get (Variables|Default|SetIntereact%20Actor (.HitActor (Collision|BreakHitResult _outhit))))
      (bind _interactiontext (Class|BPIInteraction|GetInteractData(Message) _output_get))
      (Default|Update-WBInteraction (Variables|Default|GetAs%20WB%20Interaction) true _interactiontext)
      (else
        (Variables|Default|GetIntereact%20Actor :!label _label
          (:then
            (Variables|Default|SetIntereact%20Actor 0)
            (Default|Update-WBInteraction (Variables|Default|GetAs%20WB%20Interaction) false))
          (:else))))
    (else
      (goto _label))))