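; Interactable button actor that toggles its color between green and red when used.
; The Interact event calls SV_Effect only when its ServerInteract flag is true.
; SV_Effect uses a FlipFlop to swap the Button component's material between M_Green and M_Red, starting with green, and triggers no other gameplay logic.
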(event Custom|SV_Effect
  (bind _button (Variables|Default|GetButton))
  (Utilities|FlowControl|FlipFlop
    (:A
      (Rendering|Material|SetMaterial _button 0 "/Game/ChassingTwilight/Art/Materials/M_Green.M_Green"))
    (:B
      (Rendering|Material|SetMaterial _button 0 "/Game/ChassingTwilight/Art/Materials/M_Red.M_Red"))))

(event EventBeginPlay
  (|CallParentFunction) ; This node is disabled and will not be called.\nDrag off pins to build functionality.
)

(event Collision|EventActorBeginOverlap
  (params (OtherActor :type Actor%20Object%20Reference))
  (|CallParentFunction OtherActor) ; This node is disabled and will not be called.\nDrag off pins to build functionality.
)

(event EventTick
  (params (DeltaSeconds :type Float%20%28single-precision%29))
  (|CallParentFunction DeltaSeconds) ; This node is disabled and will not be called.\nDrag off pins to build functionality.
)

(event EventInteract
  (params (PlayerThatInteracts :type Actor%20Object%20Reference) (ServerInteract? :type Boolean))
  (if ServerInteract?
    (CallFunction|SVEffect)))

(fn ConstructionScript
  (|CallParentFunction))